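; Day-night cycle controller that advances a game clock and drives the sun, sky light and sky sphere.
; The construction script seeds time from Day, Hour, Minute and Second and applies the lighting immediately.
; A looping timer, with its interval derived from Speed, advances time and samples hour-based curves for sun pitch, light intensities and sky light color.
; Tick prints the current day and time on screen.
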(event Custom|ChangeTime
  (Variables|System|SetTime (+ (Variables|System|GetTime) (* (Servise|GetTimerRate) (Variables|Settings|GetSpeed))))
  (System|Update))

(event EventBeginPlay
  (Utilities|Time|SetTimerbyEvent (delegate Custom|ChangeTime) (Servise|GetTimerRate) true))

(event EventTick
  (params (DeltaSeconds :type Float%20%28single-precision%29))
  (Debag|DisplayTime))

(fn ConstructionScript
  ;[1 1 1] инициализируем Time
  (Variables|System|SetTime (+ (* (Variables|Default|GetDay) 8.64e+04) (* (Variables|Default|GetHour) 3.6e+03) (* (Variables|Default|GetMinute) 6e+01) (Math|Conversions|ToFloat(Integer) (Variables|Default|GetSecond))))
  (System|Update))

(fn GetTimerRate
  ;[0 1 0.2845] Изменения качаемы частоты таймера
  (return (Math|Float|Max(Float) (/ 1.0 (Variables|Settings|GetSpeed)) 0.01)))

(fn GetHour
  ;[1 0 0.2429] Узнаем время на данный момент
  (return (/ (Math|Float|%(Float) (Variables|System|GetTime) 8.64e+04) 3.6e+03)))

(fn GetTimeSpan
  ;[1 0.1703 0.8771] Получить день, часы, секунды
  (return (Math|Timespan|MakeTimespan 0 0 0 (Math|Float|Truncate (Variables|System|GetTime)))))

(fn DisplayTime
  (bind _timespan (CallFunction|GetTimeSpan))
  (Development|PrintText (Utilities|Text|FormatText "День {day}: {h}: {m}: {s} " (.days _timespan) (Utilities|Text|ToText(Integer) (.hours _timespan) false true 2 3) (Utilities|Text|ToText(Integer) (.minutes _timespan) false true 2 3) (Utilities|Text|ToText(Integer) (.seconds _timespan) false true 2 3)) true true "(R=0.000000,G=0.729167,B=0.117491,A=1.000000)" 0.0))

(fn Update
  (Transformation|SetActorRotation (Variables|Settings|Objects|GetDirLight) (Math|Rotator|MakeRotator 0.0 (Math|Curves|GetFloatValue (Variables|Settings|Curves|GetCurveDirLightPitch) (CallFunction|GetHour)) 0.0))
  (Rendering|Components|Light|SetIntensity (Variables|/Script/Engine.Light|GetLightComponent (Variables|Settings|Objects|GetDirLight)) (Math|Curves|GetFloatValue (Variables|Settings|Curves|GetCurveDirLightItensity) (CallFunction|GetHour)))
  (Rendering|Components|Light|SetIntensity (Variables|/Script/Engine.SkyLight|GetLightComponent (Variables|Settings|Objects|GetSkyLight)) (Math|Curves|GetFloatValue (Variables|Settings|Curves|GetCurveSkyLightIntensity) (CallFunction|GetHour)))
  (Rendering|Components|Light|SetLightColor (Variables|/Script/Engine.SkyLight|GetLightComponent (Variables|Settings|Objects|GetSkyLight)) (Math|Curves|GetLinearColorValue (Variables|Settings|Curves|GetCurveSkyLightColor) (CallFunction|GetHour)))
  (Default|UpdateSunDirection (Variables|Settings|Objects|GetSkySphere)))